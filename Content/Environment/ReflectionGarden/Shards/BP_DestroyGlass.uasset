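; BP_DestroyGlass is an overlap actor in the Reflection Garden that destroys any BP_ClickableShard that touches it.
; ActorBeginOverlap casts the other actor to the shard class, destroys it, waits a second, then resets and increments EscapeTick, leaving it at one.
; Disconnected leftover nodes for dialogue display, an overlay material fade and BP_ClickableObject spawning never execute.
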(event `self.ReceiveActorBeginOverlap`
  (params (OtherActor :type "Actor Object Reference"))
  (bind _asbp_clickable_shard (cast `/Game/Environment/ReflectionGarden/Shards/BP_ClickableShard` OtherActor))
  (`self.K2_DestroyActor` _asbp_clickable_shard)
  (`KismetSystemLibrary.Delay` 1.0)
  (bind _output_get (set `self.EscapeTick` 0))
  (`/Engine/EditorBlueprintResources/StandardMacros.IncrementInt` _output_get))

(fn `UserConstructionScript`)