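; Player-controlled 2D side-scrolling character that moves along the world X axis and jumps, using a Paper2D flipbook sprite.
; BeginPlay adds the 2D Enhanced Input mapping context, whose actions drive movement and jumping.
; Tick flips the sprite by yaw to match horizontal velocity and sets its flipbook when two sprite counters match.
; GetFrame and the movement-updated event are empty stubs.
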(event `self.ReceiveBeginPlay`
  (bind _returnvalue (pcsubsystem `EnhancedInputLocalPlayerSubsystem` (`GameplayStatics.GetPlayerController` 0)))
  (`/Engine/EditorBlueprintResources/StandardMacros.IsValid` _returnvalue
    (:`Is Valid`
      (`EnhancedInputSubsystemInterface.AddMappingContext` _returnvalue "/Game/Environment/Characters/IMC_CharacterInput2D.IMC_CharacterInput2D" 0 (struct)))))

(event `EnhancedInput|/Game/Environment/Characters/IA_Move2D`
  (params (ActionValue :type "Float (double-precision)") (ElapsedSeconds :type "Float (double-precision)") (TriggeredSeconds :type "Float (double-precision)") (InputAction :type "InputAction Object Reference" :default "/Game/Environment/Characters/IA_Move2D.IA_Move2D"))
  (:`Triggered`
    (`self.AddMovementInput` (1.0 0.0 0.0) ActionValue)))

(event `self.ReceiveTick`
  (params (DeltaSeconds :type "Float (single-precision)"))
  (`self.UpdateCharcterRotation`)
  (if (== (`self.SpriteCount_Previous`) (`self.SpriteCount`))
    (`PaperFlipbookComponent.SetFlipbook` (`self.Sprite`) (`self.SpriteArray`))
    (set `self.SpriteCount_Previous` 1)))

(event `UpdateCharcterRotation`
  (bind _sprite (`self.Sprite`))
  (bind _velocity_x (`KismetMathLibrary.BreakVector` (`MovementComponent.Velocity` (`self.CharacterMovement`))))
  (`/Engine/EditorBlueprintResources/StandardMacros.CompareFloat` _velocity_x
    (:`>`
      (`SceneComponent.K2_SetRelativeRotation` :`self` _sprite))
    (:`<`
      (`SceneComponent.K2_SetRelativeRotation` _sprite (struct :`Yaw` 180.0) false false))))

(event `OnCharacterMovementUpdated_Event`
  (params (DeltaSeconds :type "Float (single-precision)") (OldLocation :type "Vector Structure") (OldVelocity :type "Vector Structure")))

(event `EnhancedInput|/Game/Environment/Characters/IA_Jump2D`
  (params (ActionValue :type "Float (double-precision)") (ElapsedSeconds :type "Float (double-precision)") (TriggeredSeconds :type "Float (double-precision)") (InputAction :type "InputAction Object Reference" :default "/Game/Environment/Characters/IA_Jump2D.IA_Jump2D"))
  (:`Triggered`
    (`self.Jump`)))

(fn `GetFrame`)

(fn `UserConstructionScript`)