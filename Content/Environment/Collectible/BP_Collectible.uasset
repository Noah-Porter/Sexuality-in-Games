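; Clickable collectible actor that opens an interaction widget when clicked.
; On click it limits its SceneCaptureComponent2D to its own components, adds WB_InteractWithObject to the viewport and sets SpriteCount to 1 on the player's BP_MyChar.
; A Rotate function yaws the root slightly, but its looping timer is never triggered, and the Collectible function is empty.
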(event `self.ReceiveBeginPlay`)

(event `self.ReceiveActorOnClicked`
  (params (ButtonPressed :type "Key Structure"))
  (`SceneCaptureComponent.ShowOnlyActorComponents` (`self.SceneCaptureComponent2D`) self false)
  (bind _returnvalue (`|CreateWidget` "/Game/Environment/Dialogue/WB_InteractWithObject.WB_InteractWithObject_C"))
  (bind _output_get (set `self.3D_Widget` _returnvalue))
  (`UserWidget.AddToViewport` _output_get 0)
  (bind _asbp_my_char (cast `/Game/Environment/Characters/BP_MyChar` (`GameplayStatics.GetPlayerPawn` 0)))
  (set `/Game/Environment/Characters/BP_MyChar.SpriteCount` 1 _asbp_my_char))

(fn `Collectible`)

(fn `Rotate`
  (`SceneComponent.K2_AddLocalRotation` (`self.DefaultSceneRoot`) (`KismetMathLibrary.MakeRotator` 0.0 0.0 0.5) false false))

(fn `UserConstructionScript`)