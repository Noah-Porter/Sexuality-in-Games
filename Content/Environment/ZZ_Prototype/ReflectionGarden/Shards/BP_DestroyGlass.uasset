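; Overlap trigger in the Reflection Garden prototype that checks the player's shard-hunt progress and moves them to the next level.
; When BP_ThirdPersonCharacter enters, an EscapeTick of 4 prints a completion message and, after a delay, opens Mirrors_2D.
; Other non-zero counts print delayed encouragement; this graph never changes the counter.
; Unconnected leftover chains hold dialogue-widget, fade-material and clickable-object spawning logic.
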(event `self.ReceiveActorBeginOverlap`
  (params (OtherActor :type "Actor Object Reference"))
  (cast `/Game/ThirdPerson/Blueprints/BP_ThirdPersonCharacter` OtherActor)
  (if (== (`self.EscapeTick`) 4)
    (`KismetSystemLibrary.PrintText` "You have found all of the shards. What do they show?")
    (`KismetSystemLibrary.Delay` 3.0)
    (`GameplayStatics.OpenLevel` "Mirrors_2D")
    (elif (not (== (`self.EscapeTick`) 0))
      (`KismetSystemLibrary.Delay` 1.0)
      (`KismetSystemLibrary.PrintText` "Good work, almost there!"))))

(fn `UserConstructionScript`)