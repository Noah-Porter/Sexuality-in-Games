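; BP_Nuance is a prototype NPC that shows dialogue and can be sent toward the player.
; Each Talk call advances an index into the Dialogue array, showing the line in a lazily created WB_Dialogue widget and removing it past the end.
; Pressing E starts AI MoveTo toward the character's CurrentLocation, whose immediate exec output casts the player and loops straight back without waiting for completion.
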(event `self.Talk`
  (`/Engine/EditorBlueprintResources/StandardMacros.IncrementInt` (`self.talkindex`)
    (:`  `
      (if (< (`self.talkindex`) (`KismetArrayLibrary.Array_Length` (`self.dialogue`)))
        (`self.UI`
          (:`then`
            _)
          (:`else`
            (bind _returnvalue (`|CreateWidget` "/Game/Dialogue/WB_Dialogue.WB_Dialogue_C" (`GameplayStatics.GetPlayerController` 0)))
            (bind _output_get (set `self.UI` _returnvalue))
            (`UserWidget.AddToViewport` _output_get 0)))
        (`TextBlock.SetText` (`/Game/Dialogue/WB_Dialogue.TalkText` (`self.UI`)) (`KismetTextLibrary.Conv_StringToText` (`|GetArrayItem` (`self.dialogue`) (`self.talkindex`))))
        (else
          (`Widget.RemoveFromParent` (`self.UI`)))))))

(event `Key|E`
  (params (Key :type "Key Structure"))
  (:`Pressed`
    (`AITask_MoveTo.AIMoveTo` (`AIBlueprintHelperLibrary.GetAIController` null) (`/Game/ThirdPerson/Blueprints/BP_ThirdPersonCharacter.CurrentLocation` (stale _asbp_third_person_character)) null -1.0 "Default" "Default" true true true :!label _label
      (:`then`
        (bind _asbp_third_person_character (cast `/Game/ThirdPerson/Blueprints/BP_ThirdPersonCharacter` (`GameplayStatics.GetPlayerCharacter` 0)))
        (goto _label)))))

(fn `UserConstructionScript`)