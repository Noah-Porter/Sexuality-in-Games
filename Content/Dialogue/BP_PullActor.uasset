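; BP_PullActor is an actor that moves itself through a PullTowardsTarget event, which nothing in this file calls.
; The event applies a local-space, non-sweeping offset along the normalized direction from the player character to BPNPC's owner, scaled by Speed and frame delta.
; Overlap events compare the other actor to the player controller, then set or clear an OtherActor reference that the pull never reads.
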(event `self.ReceiveActorBeginOverlap`
  (params (OtherActor :type "Actor Object Reference"))
  (if (== OtherActor (`GameplayStatics.GetPlayerController` 0))
    (set `self.Other Actor` OtherActor)))

(event `self.ReceiveActorEndOverlap`
  (params (OtherActor :type "Actor Object Reference"))
  (if (== OtherActor (`GameplayStatics.GetPlayerController` 0))
    (set `self.Other Actor` null)))

(event `PullTowardsTarget`
  (`self.K2_AddActorLocalOffset` (* (`KismetMathLibrary.Normal` (- (`self.K2_GetActorLocation` (`ActorComponent.GetOwner` (`self.BP_NPC`))) (`self.K2_GetActorLocation` (`GameplayStatics.GetPlayerCharacter` 0)))) (`GameplayStatics.GetWorldDeltaSeconds`) (`self.Speed`))))

(fn `UserConstructionScript`)